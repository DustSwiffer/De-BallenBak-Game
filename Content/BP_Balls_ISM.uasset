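; BP_Balls_ISM is an actor that scatters small balls using instanced static meshes.
; On BeginPlay it creates one movable instanced mesh component per entry in BallMaterials, assigning the sphere mesh and that material.
; Each component has physics simulation enabled and ignores the Pawn channel.
; A loop driven by BallsCount then fills each component with scaled-down instances at random positions over a low, wide area.
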(event EventBeginPlay
  (for (_array_element _array_index) (Variables|Default|GetBallMaterials)
    (Utilities|FlowControl|Sequence
      (:then_0
        ;[0.01938 0.01938 0.01938] Set Mesh
        (bind _returnvalue (AddComponent|AddInstancedStaticMeshComponent false))
        (Collision|SetCollisionResponsetoChannel _returnvalue "ECC_Pawn" "ECR_Ignore")
        (Physics|SetSimulatePhysics _returnvalue true)
        (Transformation|SetMobility _returnvalue "Movable")
        (Rendering|Material|SetMaterial _returnvalue 0 _array_element)
        (Utilities|Array|Add (Variables|Default|GetISMs) _returnvalue)
        (Components|StaticMesh|SetStaticMesh _returnvalue "/Game/StarterContent/Props/MaterialSphere.MaterialSphere"))
      (:then_1
        (for _index (range 0 (Variables|Default|GetBallsCount))
          (Components|InstancedStaticMesh|AddInstance (Utilities|Array|Get(acopy) (Variables|Default|GetISMs) _array_index) (Math|Transform|MakeTransform (Math|Vector|MakeVector (Math|Random|RandomFloatinRange 3e+01 1.5e+03) (Math|Random|RandomFloatinRange 3e+01 1.5e+03) (Math|Random|RandomFloatinRange 0.0 3e+01)) "0, 0, 0" (Math|Vector|MakeVector 0.25 0.25 0.25)) false))))))

(fn ConstructionScript)